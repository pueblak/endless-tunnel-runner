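; BP_Projectile is a projectile that damages players and kills enemies on contact.
; Each tick it moves itself by a swept world offset from its Velocity, with no movement component in the logic.
; On collision overlap it ignores its Source, deals 1 damage to BP_Player or destroys BP_Enemy outright, then destroys itself.
; Overlaps with other actor types leave it alive.
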(event `self.ReceiveTick`
  (params (DeltaSeconds :type "Float (single-precision)"))
  (`self.K2_AddActorWorldOffset` (* (`self.Velocity`) DeltaSeconds) true))

(event `self.Collision.OnComponentBeginOverlap`
  (params (OverlappedComponent :type "PrimitiveComponent Object Reference") (OtherActor :type "Actor Object Reference") (OtherComp :type "PrimitiveComponent Object Reference") (OtherBodyIndex :type Integer) (bFromSweep :type Boolean) (SweepResult :type "HitResult Structure (by ref)"))
  (if (not (== (`self.Source`) OtherActor))
    (bind _asbp_player (cast `/Game/InfiniteMatrix/Blueprints/BP_Player` OtherActor)
      (:`then`
        (`/Game/InfiniteMatrix/Blueprints/BP_Player.Damage` _asbp_player 1))
      (:`CastFailed`
        (bind _asbp_enemy (cast `/Game/InfiniteMatrix/Blueprints/BP_Enemy` OtherActor))
        (`self.K2_DestroyActor` _asbp_enemy)))
    (`self.K2_DestroyActor`)))

(fn `UserConstructionScript`)