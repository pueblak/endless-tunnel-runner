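; BP_TunnelSpawner builds a chain of BP_Tunnel segments, each with randomized walls, enemies and pickups.
; On BeginPlay it clears existing tunnels, then spawns a starting run at zero difficulty from the player pawn's location.
; Each new segment attaches at the newest tunnel's SpawnPoint, alternates HasWall and stores a reference back to the spawner.
; Difficulty feeds wall and enemy randomization and quadratically shrinks the maximum pickup count as it rises toward eight.
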(event `self.ReceiveBeginPlay`
  (`self.SpawnInitialTunnels`))

(fn `SpawnInitialTunnels`
  (`|ExecutionSequence`
    (:`then_0`
      (bind _outactors (`GameplayStatics.GetAllActorsOfClass` "/Game/InfiniteMatrix/Blueprints/BP_Tunnel.BP_Tunnel_C"))
      (for _array_element _outactors
        (`self.K2_DestroyActor` _array_element)))
    (:`then_1`
      (for _ (range 6)
        (`/Engine/EditorBlueprintResources/StandardMacros.IsValid` (`self.NewestTunnel`)
          (:`Is Valid`
            (`self.SpawnTunnelAtSpawnPoint` 0))
          (:`Is Not Valid`
            (`self.SpawnTunnel` (`self.K2_GetActorLocation` (`GameplayStatics.GetPlayerPawn` 0)))))))))

(fn `SpawnTunnel`
  (params (SpawnLocation :type "Vector Structure") (HasWall :type Boolean) (Difficulty :type Integer))
  (bind _returnvalue (`KismetMathLibrary.Conv_IntToDouble` (- 8 Difficulty)))
  (bind _returnvalue_2 (`|SpawnActorFromClass` "/Game/InfiniteMatrix/Blueprints/BP_Tunnel.BP_Tunnel_C" (`KismetMathLibrary.MakeTransform` SpawnLocation) "Undefined" "OverrideRootScale" null null))
  (set `/Game/InfiniteMatrix/Blueprints/BP_Tunnel.HasWall` HasWall _returnvalue_2)
  (bind _output_get (set `self.NewestTunnel` _returnvalue_2))
  (set `/Game/InfiniteMatrix/Blueprints/BP_Tunnel.TunnelSpawner` self _output_get)
  (`/Game/InfiniteMatrix/Blueprints/BP_Tunnel.RandomizeWall` _returnvalue_2 Difficulty)
  (`/Game/InfiniteMatrix/Blueprints/BP_Tunnel.RandomizeEnemies` _returnvalue_2 (/ (+ Difficulty 1) 2))
  (`/Game/InfiniteMatrix/Blueprints/BP_Tunnel.RandomizePickups` _returnvalue_2 (`KismetMathLibrary.RandomIntegerInRange` 0 (`KismetMathLibrary.FFloor` (+ (`KismetMathLibrary.RandomFloat`) (/ (* _returnvalue _returnvalue) 29.0)))) 0.625 0.25 0.125))

(fn `SpawnTunnelAtSpawnPoint`
  (params (Difficulty :type Integer))
  (bind _newesttunnel (`self.NewestTunnel`))
  (`self.SpawnTunnel` (`SceneComponent.K2_GetComponentLocation` (`/Game/InfiniteMatrix/Blueprints/BP_Tunnel.SpawnPoint` _newesttunnel)) (not (`/Game/InfiniteMatrix/Blueprints/BP_Tunnel.HasWall` _newesttunnel)) Difficulty))

(fn `UserConstructionScript`)