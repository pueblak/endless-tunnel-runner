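; BP_Tunnel is a tunnel segment for an endless runner, optionally holding a rotating wall with a hole.
; RandomizeWall picks a hole mesh (none without a wall), start roll and spin speed, which Tick applies.
; When the player overlaps TriggerZone, the segment asks TunnelSpawner for another, destroys itself and, if walled, awards score, setting the player's SpeedIncrement at a milestone.
; Hitting the wall costs health and score, or kills a low-health player.
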(event `self.ReceiveTick`
  (params (DeltaSeconds :type "Float (single-precision)"))
  (`SceneComponent.K2_AddLocalRotation` (`self.WallMesh`) (`KismetMathLibrary.MakeRotator` (* DeltaSeconds (`self.RotateSpeed`))) false false))

(event `self.TriggerZone.OnComponentBeginOverlap`
  (params (OverlappedComponent :type "PrimitiveComponent Object Reference") (OtherActor :type "Actor Object Reference") (OtherComp :type "PrimitiveComponent Object Reference") (OtherBodyIndex :type Integer) (bFromSweep :type Boolean) (SweepResult :type "HitResult Structure (by ref)"))
  (bind _asbp_player (cast `/Game/InfiniteMatrix/Blueprints/BP_Player` OtherActor))
  (`/Game/InfiniteMatrix/Blueprints/BP_TunnelSpawner.SpawnTunnelAtSpawnPoint` (`self.TunnelSpawner`))
  (`self.K2_DestroyActor`)
  (if (`self.HasWall`)
    (bind _output_get (set `/Game/InfiniteMatrix/Blueprints/BP_Player.Score` (+ (`/Game/InfiniteMatrix/Blueprints/BP_Player.Score` _asbp_player) 1) _asbp_player))
    (`/Game/InfiniteMatrix/Blueprints/BP_Player.UpdateScore` _asbp_player)
    (if (== _output_get 60)
      (set `/Game/InfiniteMatrix/Blueprints/BP_Player.SpeedIncrement` 50.0 _asbp_player))))

(event `self.WallMesh.OnComponentHit`
  (params (HitComponent :type "PrimitiveComponent Object Reference") (OtherActor :type "Actor Object Reference") (OtherComp :type "PrimitiveComponent Object Reference") (NormalImpulse :type "Vector Structure") (Hit :type "HitResult Structure (by ref)"))
  (bind _asbp_player (cast `/Game/InfiniteMatrix/Blueprints/BP_Player` OtherActor))
  (bind _health (`/Game/InfiniteMatrix/Blueprints/BP_Player.Health` _asbp_player))
  (if (> 3 _health)
    (set `/Game/InfiniteMatrix/Blueprints/BP_Player.IsDead` true _asbp_player)
    (`/Game/InfiniteMatrix/Blueprints/BP_Player.UpdateHealth` _asbp_player 0 0)
    (`/Game/InfiniteMatrix/Blueprints/BP_Player.DisplayRestart` _asbp_player)
    (else
      (`/Game/InfiniteMatrix/Blueprints/BP_Player.UpdateHealth` _asbp_player (- _health 2) 0)
      (`PrimitiveComponent.SetCollisionEnabled` HitComponent "NoCollision")
      (set `/Game/InfiniteMatrix/Blueprints/BP_Player.Score` (- (`/Game/InfiniteMatrix/Blueprints/BP_Player.Score` _asbp_player) 1) _asbp_player))))

(fn `RandomizeWall`
  (`StaticMeshComponent.SetStaticMesh` (`self.WallMesh`) (select `int` (`KismetMathLibrary.SelectInt` (`KismetMathLibrary.RandomIntegerInRange` 0 3) 4 (`self.HasWall`)) :`0` "/Game/InfiniteMatrix/Meshes/SM_Hole_01.SM_Hole_01" :`1` "/Game/InfiniteMatrix/Meshes/SM_Hole_02.SM_Hole_02" :`2` "/Game/InfiniteMatrix/Meshes/SM_Hole_03.SM_Hole_03" :`3` "/Game/InfiniteMatrix/Meshes/SM_Hole_04.SM_Hole_04" :`4` null :!type "StaticMesh Object Reference"))
  (`SceneComponent.K2_AddLocalRotation` (`self.WallMesh`) (`KismetMathLibrary.MakeRotator` (`KismetMathLibrary.RandomFloatInRange` 0.0 360.0)) false false)
  (set `self.RotateSpeed` (select `int` (`KismetMathLibrary.RandomIntegerInRange` 0 5) :`0` 30.0 :`1` 60.0 :`2` 90.0 :`3` -30.0 :`4` -60.0 :`5` -90.0 :!type "Float (single-precision)")))

(fn `UserConstructionScript`)