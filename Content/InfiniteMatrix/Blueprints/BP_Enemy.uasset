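; BP_Enemy is an enemy actor that deals damage to BP_Player on collision overlap, then destroys itself.
; FireProjectile spawns a half-scale BP_Projectile with itself as Source, moving at ProjectileSpeed toward a point on the world X axis, 1000 units toward -X from EnemyBody.
; The spawn location is that direction scaled, without adding the body's position.
; Nothing in this graph calls FireProjectile.
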(event `self.ReceiveTick`
  (params (DeltaSeconds :type "Float (single-precision)")))

(event `self.Collision.OnComponentBeginOverlap`
  (params (OverlappedComponent :type "PrimitiveComponent Object Reference") (OtherActor :type "Actor Object Reference") (OtherComp :type "PrimitiveComponent Object Reference") (OtherBodyIndex :type Integer) (bFromSweep :type Boolean) (SweepResult :type "HitResult Structure (by ref)"))
  (bind _asbp_player (cast `/Game/InfiniteMatrix/Blueprints/BP_Player` OtherActor))
  (`/Game/InfiniteMatrix/Blueprints/BP_Player.Damage` _asbp_player 2)
  (`self.K2_DestroyActor`))

(fn `FireProjectile`
  (bind (_returnvalue_x _returnvalue_y _returnvalue_z) (`KismetMathLibrary.BreakVector` (`SceneComponent.K2_GetComponentLocation` (`self.EnemyBody`))))
  (bind _returnvalue (`KismetMathLibrary.GetDirectionUnitVector` (`KismetMathLibrary.MakeVector` _returnvalue_x _returnvalue_y _returnvalue_z) (+ (`KismetMathLibrary.MakeVector` _returnvalue_x) (-1000.0 0.0 0.0))))
  (bind _returnvalue_2 (`|SpawnActorFromClass` "/Game/InfiniteMatrix/Blueprints/BP_Projectile.BP_Projectile_C" (`KismetMathLibrary.MakeTransform` (* _returnvalue 100.0) (struct) (0.5 0.5 0.5)) "AdjustIfPossibleButAlwaysSpawn" "OverrideRootScale" null null))
  (set `/Game/InfiniteMatrix/Blueprints/BP_Projectile.Velocity` (* _returnvalue (`self.ProjectileSpeed`)) _returnvalue_2)
  (set `/Game/InfiniteMatrix/Blueprints/BP_Projectile.Source` self _returnvalue_2))

(fn `UserConstructionScript`)